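; BP_DropArea is a drop target in the drag-and-drop system that receives dropped content.
; TryDropContent fails when the Ocupado (occupied) flag is set, otherwise it stores the content, increments the stack count and returns true.
; A StackLimit check exists but is disconnected and never runs, and nothing in these graphs sets Ocupado.
; The event graph and construction script are empty.
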(fn `TryDropContent`
  (params (ObjectContent :type "/Game/DragAndDropSystem/I_Draggable Interface"))
  (returns (DroppedIn :type Boolean))
  (if (`self.Ocupado`)
    ;[1 0.474 0.474] Fail Bc ocupado
    (return false)
    (else
      (set `self.Content` ObjectContent)
      (`/Engine/EditorBlueprintResources/StandardMacros.IncrementInt` (`self.CurrentStackAmount`)
        (:`  `
          (return true))))))

(fn `UserConstructionScript`)